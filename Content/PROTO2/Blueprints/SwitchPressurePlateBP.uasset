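; Pressure plate switch that toggles two linked doors in opposite states.
; Beginning overlap opens Door1 and closes Door2 by setting their IsOpen flags, and ending overlap reverses them.
; Both events call PressurePlateDown, which snaps the plate actor to CloseLoc and plays a laser door sound.
; PressurePlateUp, which moves it to OpenLoc with a closing sound, is not called in this graph.
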(event `self.ReceiveActorEndOverlap`
  (params (OtherActor :type "Actor Object Reference"))
  (set `/Game/PROTO2/Blueprints/DoorBP.IsOpen` false (`self.Door1`))
  (set `/Game/PROTO2/Blueprints/DoorBP.IsOpen` true (`self.Door2`))
  (`self.PressurePlateDown`))

(event `self.ReceiveActorBeginOverlap`
  (params (OtherActor :type "Actor Object Reference"))
  (set `/Game/PROTO2/Blueprints/DoorBP.IsOpen` true (`self.Door1`))
  (set `/Game/PROTO2/Blueprints/DoorBP.IsOpen` false (`self.Door2`))
  (`self.PressurePlateDown`))

(fn `PressurePlateDown`
  (`self.K2_SetActorLocation` (`self.PressurePlate`) (`self.CloseLoc`) false false)
  (`GameplayStatics.PlaySoundAtLocation` "/Game/Audio/Laser_door_open.Laser_door_open" (`SceneComponent.K2_GetComponentLocation` (`self.DefaultSceneRoot`)) (struct) 0.5 1.0 0.0 null null null))

(fn `PressurePlateUp`
  (`self.K2_SetActorLocation` (`self.PressurePlate`) (`self.OpenLoc`) false false)
  (`GameplayStatics.PlaySoundAtLocation` "/Game/Audio/Laserdoorclose.Laserdoorclose" (`SceneComponent.K2_GetComponentLocation` (`self.DefaultSceneRoot`)) (struct) 0.5 1.0 0.0 null null null))

(fn `UserConstructionScript`)