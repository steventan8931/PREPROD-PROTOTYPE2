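; SecurityCamColliderBP is a trigger actor that lets the player take control of a linked security camera pawn.
; It counts overlapping actors, and when the count is at most one on begin overlap, enables camera control on PlayerBP1 and assigns it the CameraPawn.
; It also gives the SecurityCameraPawnBP a reference back to the player pawn.
; End overlap only decrements the count, as the logic revoking camera control is disconnected.
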(event `self.ReceiveActorEndOverlap`
  (params (OtherActor :type "Actor Object Reference"))
  (bind _result (`/Engine/EditorBlueprintResources/StandardMacros.DecrementInt` (`self.ActorsColliding`))
    (:`  `
      (set `self.ActorsColliding` _result))))

(event `self.ReceiveActorBeginOverlap`
  (params (OtherActor :type "Actor Object Reference"))
  (bind _result (`/Engine/EditorBlueprintResources/StandardMacros.IncrementInt` (`self.ActorsColliding`))
    (:`  `
      (bind _output_get (set `self.ActorsColliding` _result))
      (if (<= _output_get 1)
        (bind _asplayer_bp1 (cast `/Game/PROTO2/Blueprints/PlayerBP1` OtherActor))
        (set `/Game/PROTO2/Blueprints/PlayerBP1.CanControlCamera` true _asplayer_bp1)
        (set `/Game/PROTO2/Blueprints/PlayerBP1.Camera` (`self.CameraPawn`) _asplayer_bp1)
        (bind _assecurity_camera_pawn_bp (cast `/Game/PROTO2/Blueprints/SecurityCameraPawnBP` (`self.CameraPawn`)))
        (set `/Game/PROTO2/Blueprints/SecurityCameraPawnBP.PlayerPawn` (`PawnMovementComponent.GetPawnOwner` (`Character.CharacterMovement` _asplayer_bp1)) _assecurity_camera_pawn_bp)))))

(fn `UserConstructionScript`)