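; PoisonGasBP is a poison gas volume actor that flags the player as being in gas while overlapping it.
; Begin and end overlap cast the other actor to PlayerBP1 and set its InGas flag true or false.
; On BeginPlay it finds the SecurityCameraPawnBP, stores it as Camera and makes it its owner.
; It applies no damage itself, and a mask check and delay are left unused.
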(event `self.ReceiveBeginPlay`
  (bind _returnvalue (`GameplayStatics.GetActorOfClass` "/Game/PROTO2/Blueprints/SecurityCameraPawnBP.SecurityCameraPawnBP_C"))
  (set `self.Camera` _returnvalue)
  (`self.SetOwner` (`self.Camera`)))

(event `self.ReceiveActorEndOverlap`
  (params (OtherActor :type "Actor Object Reference"))
  (bind _asplayer_bp1 (cast `/Game/PROTO2/Blueprints/PlayerBP1` OtherActor))
  (set `/Game/PROTO2/Blueprints/PlayerBP1.InGas` false _asplayer_bp1))

(event `self.ReceiveActorBeginOverlap`
  (params (OtherActor :type "Actor Object Reference"))
  (bind _asplayer_bp1 (cast `/Game/PROTO2/Blueprints/PlayerBP1` OtherActor))
  (set `/Game/PROTO2/Blueprints/PlayerBP1.InGas` true _asplayer_bp1))

(event `self.ReceiveTick`
  (params (DeltaSeconds :type "Float (single-precision)")))

(fn `UserConstructionScript`)