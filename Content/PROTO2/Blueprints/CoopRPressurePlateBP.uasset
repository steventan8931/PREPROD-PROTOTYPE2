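; Right-hand co-op pressure plate that reports to a referenced Door whether it is being stood on.
; Any actor overlap sets the Door's IsOpenR flag and plays a pickup sound at world origin; end overlap clears it, until the Door is Opened.
; Separate PressurePlateDown and PressurePlateUp functions move the plate between two locations with laser-door sounds, but nothing in this Blueprint calls them.
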(event `self.ReceiveActorEndOverlap`
  (params (OtherActor :type "Actor Object Reference"))
  (bind _door (`self.Door`))
  (if (not (`/Game/PROTO2/Blueprints/CoopDoorBP.Opened` _door))
    (set `/Game/PROTO2/Blueprints/CoopDoorBP.IsOpenR` false _door)))

(event `self.ReceiveActorBeginOverlap`
  (params (OtherActor :type "Actor Object Reference"))
  (bind _door (`self.Door`))
  (if (not (`/Game/PROTO2/Blueprints/CoopDoorBP.Opened` _door))
    (set `/Game/PROTO2/Blueprints/CoopDoorBP.IsOpenR` true _door)
    (`GameplayStatics.PlaySoundAtLocation` "/Game/Audio/PickupItem.PickupItem" (0.0 0.0 0.0) (struct) 1.0 1.0 0.0 null null null)))

(fn `PressurePlateDown`
  (`self.K2_SetActorLocation` (`self.PressurePlate`) (`self.DownLoc`) false false)
  (`GameplayStatics.PlaySoundAtLocation` "/Game/Audio/Laser_door_open.Laser_door_open" (`SceneComponent.K2_GetComponentLocation` (`self.DefaultSceneRoot`)) (struct) 0.5 1.0 0.0 null null null))

(fn `PressurePlateUp`
  (`self.K2_SetActorLocation` (`self.PressurePlate`) (`self.OpenLoc`) false false)
  (`GameplayStatics.PlaySoundAtLocation` "/Game/Audio/Laserdoorclose.Laserdoorclose" (`SceneComponent.K2_GetComponentLocation` (`self.DefaultSceneRoot`)) (struct) 0.5 1.0 0.0 null null null))

(fn `UserConstructionScript`)