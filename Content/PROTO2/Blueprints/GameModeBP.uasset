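; GameModeBP is a game mode that detects when the players have finished, with a threshold of two.
; On BeginPlay it caches every PlayerBP1 actor in the Players array.
; Each Tick it polls their ReachedEnd flags, incrementing a running counter or zeroing it at any unfinished player.
; The counter is not reset between ticks, so "Game Finished" prints repeatedly while all players remain at the end.
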(event `self.ReceiveBeginPlay`
  (bind _outactors (`GameplayStatics.GetAllActorsOfClass` "/Game/PROTO2/Blueprints/PlayerBP1.PlayerBP1_C"))
  (set `self.Players` _outactors))

(event `self.ReceiveTick`
  (params (DeltaSeconds :type "Float (single-precision)"))
  (for _array_element (`self.Players`)
    (if (`/Game/PROTO2/Blueprints/PlayerBP1.ReachedEnd` _array_element)
      (bind _result (`/Engine/EditorBlueprintResources/StandardMacros.IncrementInt` (`self.PlayersAtEndCount`))
        (:`  `
          (bind _output_get (set `self.PlayersAtEndCount` _result))
          (if (>= _output_get 2)
            (`KismetSystemLibrary.PrintString` "Game Finished"))))
      (else
        (set `self.PlayersAtEndCount` 0)))))

(fn `UserConstructionScript`)