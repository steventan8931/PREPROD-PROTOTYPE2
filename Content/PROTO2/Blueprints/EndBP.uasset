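; EndBP is an end-zone actor that detects when players reach the finish.
; Overlapping PlayerBP1 actors get ReachedEnd set and increment PlayersFinished.
; Leaving clears that player's flag and decrements the count, then resets it to zero.
; Tick prints a "we win" debug string whenever the count is at least two.
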(event `self.ReceiveActorEndOverlap`
  (params (OtherActor :type "Actor Object Reference"))
  (bind _asplayer_bp1 (cast `/Game/PROTO2/Blueprints/PlayerBP1` OtherActor))
  (set `/Game/PROTO2/Blueprints/PlayerBP1.ReachedEnd` false _asplayer_bp1)
  (`/Engine/EditorBlueprintResources/StandardMacros.DecrementInt` (`self.PlayersFinished`)
    (:`  `
      (set `self.PlayersFinished` 0))))

(event `self.ReceiveActorBeginOverlap`
  (params (OtherActor :type "Actor Object Reference"))
  (bind _asplayer_bp1 (cast `/Game/PROTO2/Blueprints/PlayerBP1` OtherActor))
  (set `/Game/PROTO2/Blueprints/PlayerBP1.ReachedEnd` true _asplayer_bp1)
  (bind _result (`/Engine/EditorBlueprintResources/StandardMacros.IncrementInt` (`self.PlayersFinished`))
    (:`  `
      (set `self.PlayersFinished` _result))))

(event `self.ReceiveTick`
  (params (DeltaSeconds :type "Float (single-precision)"))
  (if (>= (`self.PlayersFinished`) 2)
    (`KismetSystemLibrary.PrintString` "we win")))

(fn `UserConstructionScript`)