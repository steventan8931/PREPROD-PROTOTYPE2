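; Pressure plate Blueprint that opens two linked doors while stepped on.
; Actor begin and end overlap events set IsOpen on both Door references, with no filter on the overlapping actor or count of occupants, so any exit closes both.
; The same events call helper functions that snap the PressurePlate actor down or up using hardcoded absolute world locations, not offsets from its placed position.
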(event `self.ReceiveActorEndOverlap`
  (params (OtherActor :type "Actor Object Reference"))
  (set `/Game/PROTO2/Blueprints/DoorBP.IsOpen` false (`self.Door`))
  (set `/Game/PROTO2/Blueprints/DoorBP.IsOpen` false (`self.Door2`))
  (`self.PressurePlateUp`))

(event `self.ReceiveActorBeginOverlap`
  (params (OtherActor :type "Actor Object Reference"))
  (set `/Game/PROTO2/Blueprints/DoorBP.IsOpen` true (`self.Door`))
  (set `/Game/PROTO2/Blueprints/DoorBP.IsOpen` true (`self.Door2`))
  (`self.PressurePlateDown`))

(fn `PressurePlateDown`
  (`self.K2_SetActorLocation` (`self.PressurePlate`) (0.0 0.0 -10.0) false false))

(fn `PressurePlateUp`
  (`self.K2_SetActorLocation` (`self.PressurePlate`) (0.0 0.0 0.0) false false))

(fn `UserConstructionScript`)