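; GasMaskBP is a pickup actor that gives the player a gas mask from a limited supply.
; On overlap with a PlayerBP1 that has no mask, it sets the player's HasMask flag and decrements GasMasksRemaining.
; Tick checks the count every frame and, once none remain, destroys the referenced GasMask actor and then itself.
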(event `self.ReceiveActorBeginOverlap`
  (params (OtherActor :type "Actor Object Reference"))
  (bind _asplayer_bp1 (cast `/Game/PROTO2/Blueprints/PlayerBP1` OtherActor))
  (if (not (`/Game/PROTO2/Blueprints/PlayerBP1.HasMask` _asplayer_bp1))
    (set `/Game/PROTO2/Blueprints/PlayerBP1.HasMask` true _asplayer_bp1)
    (set `self.GasMasksRemaining` (- (`self.GasMasksRemaining`) 1))))

(event `self.ReceiveTick`
  (params (DeltaSeconds :type "Float (single-precision)"))
  (if (<= (`self.GasMasksRemaining`) 0)
    (`self.K2_DestroyActor` (`self.GasMask`))
    (`self.K2_DestroyActor`)))

(fn `UserConstructionScript`)