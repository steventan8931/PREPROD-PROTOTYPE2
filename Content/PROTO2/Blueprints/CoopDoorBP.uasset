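; CoopDoorBP is a double door that slides open once both its IsOpenL and IsOpenR flags are true, which are not set within this Blueprint.
; Tick raises DoorAlpha in fixed per-frame steps and calls Open, which lerps each panel from its current relative location toward its open location.
; When alpha passes the limit, Open latches Opened and plays a sound, passing the root's world scale as its location.
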(event `self.ReceiveBeginPlay`)

(event `self.ReceiveTick`
  (params (DeltaSeconds :type "Float (single-precision)"))
  (if (`self.Opened`)
    _
    (elif (and (`self.IsOpenR`) (`self.IsOpenL`))
      (set `self.DoorAlpha` (+ (`self.DoorAlpha`) 0.1))
      (`self.Open`))))

(fn `Open`
  (if (<= (`self.DoorAlpha`) 1.1)
    (`SceneComponent.K2_SetRelativeLocation` (`self.LeftDoor`) (`KismetMathLibrary.VLerp` (`SceneComponent.RelativeLocation` (`self.LeftDoor`)) (`self.OpenLocL`) (`self.DoorAlpha`)) false false)
    (`SceneComponent.K2_SetRelativeLocation` (`self.RightDoor`) (`KismetMathLibrary.VLerp` (`SceneComponent.RelativeLocation` (`self.RightDoor`)) (`self.OpenLocR`) (`self.DoorAlpha`)) false false)
    (else
      (set `self.Opened` true)
      (`GameplayStatics.PlaySoundAtLocation` "/Game/Audio/OpenDoorWithKey.OpenDoorWithKey" (`SceneComponent.K2_GetComponentScale` (`self.DefaultSceneRoot`)) (struct) 1.0 1.0 0.0 null null null))))

(fn `UserConstructionScript`)