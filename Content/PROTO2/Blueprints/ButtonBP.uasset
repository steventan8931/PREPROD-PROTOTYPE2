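; ButtonBP is an unfinished prototype button actor meant to react to a grabbing player.
; On overlap it casts the other actor to PlayerBP1 and prints a debug "open" message if either hand's grab flag is set.
; Tick checks an Open flag that nothing here sets and takes no action, while logic to offset the Cube sits disconnected and never runs.
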(event `self.ReceiveActorBeginOverlap`
  (params (OtherActor :type "Actor Object Reference"))
  (bind _asplayer_bp1 (cast `/Game/PROTO2/Blueprints/PlayerBP1` OtherActor))
  (if (or (`/Game/PROTO2/Blueprints/PlayerBP1.GrabbingL` _asplayer_bp1) (`/Game/PROTO2/Blueprints/PlayerBP1.GrabbingR` _asplayer_bp1))
    (`KismetSystemLibrary.PrintString` "open")))

(event `self.ReceiveTick`
  (params (DeltaSeconds :type "Float (single-precision)"))
  (if (`self.open`)
    _))

(fn `UserConstructionScript`)