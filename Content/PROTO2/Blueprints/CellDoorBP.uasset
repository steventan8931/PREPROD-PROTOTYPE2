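; CellDoorBP is a cell door actor that opens automatically shortly after play begins.
; On BeginPlay, a chain of delays blinks the Cube component's visibility off and on twice, then calls OpenGates.
; OpenGates deactivates and hides the Cube and disables collision on the whole actor, so the door vanishes rather than moving.
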(event `self.ReceiveBeginPlay`
  (`KismetSystemLibrary.Delay` 1.0)
  (`SceneComponent.SetVisibility` (`self.Cube`) false true)
  (`KismetSystemLibrary.Delay` 0.3)
  (`SceneComponent.SetVisibility` (`self.Cube`) true true)
  (`KismetSystemLibrary.Delay` 0.2)
  (`SceneComponent.SetVisibility` (`self.Cube`) false true)
  (`KismetSystemLibrary.Delay` 0.2)
  (`SceneComponent.SetVisibility` (`self.Cube`) true true)
  (`KismetSystemLibrary.Delay` 0.2)
  (`self.OpenGates`))

(fn `OpenGates`
  (bind _cube (`self.Cube`))
  (`ActorComponent.SetActive` _cube false true)
  (`SceneComponent.SetVisibility` _cube false true)
  (`self.SetActorEnableCollision` (`ActorComponent.GetOwner` (`self.Cube`)) false))

(fn `UserConstructionScript`)