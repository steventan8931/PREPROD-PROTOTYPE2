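; Keycard door for two players that opens when an overlapping PlayerBP1 holds a key, consuming that key.
; Open snaps Cube1 to OpenPosition, plays a sound and swaps materials on both cubes; Close runs only at BeginPlay.
; Without a key, a "keycard required" widget appears, offset horizontally for anyone other than player 0, and is removed on end overlap.
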(event `self.ReceiveBeginPlay`
  (`self.Close`))

(event `self.ReceiveActorBeginOverlap`
  (params (OtherActor :type "Actor Object Reference"))
  (bind _asplayer_bp1 (cast `/Game/PROTO2/Blueprints/PlayerBP1` OtherActor))
  (bind _collectedkey (`/Game/PROTO2/Blueprints/PlayerBP1.CollectedKey` _asplayer_bp1))
  (set `self.IsOpen` _collectedkey)
  (if _collectedkey
    (`self.Open`)
    (`Widget.RemoveFromParent` (stale `self.ReceiveActorBeginOverlap` _returnvalue))
    (set `/Game/PROTO2/Blueprints/PlayerBP1.CollectedKey` false _asplayer_bp1)
    (elif (`self.IsOpen`)
      _
      (elif (== OtherActor (`GameplayStatics.GetPlayerCharacter` 0))
        (bind _returnvalue (`|CreateWidget` "/Game/PROTO2/Blueprints/Keycard_required_widget.Keycard_required_widget_C"))
        (`UserWidget.AddToViewport` _returnvalue 0)
        (`UserWidget.SetPositionInViewport` _returnvalue (0.0 0.0) false)
        (else
          (bind _returnvalue_2 (`|CreateWidget` "/Game/PROTO2/Blueprints/Keycard_required_widget.Keycard_required_widget_C"))
          (`UserWidget.AddToViewport` _returnvalue_2 0)
          (`UserWidget.SetPositionInViewport` _returnvalue_2 (1200.0 0.0) false))))))

(event `self.ReceiveTick`
  (params (DeltaSeconds :type "Float (single-precision)")))

(event `self.ReceiveActorEndOverlap`
  (params (OtherActor :type "Actor Object Reference"))
  (if (== OtherActor (`GameplayStatics.GetPlayerCharacter` 0))
    (`/Engine/EditorBlueprintResources/StandardMacros.IsValid` (stale `self.ReceiveActorBeginOverlap` _returnvalue)
      (:`Is Valid`
        (`Widget.RemoveFromParent` (stale `self.ReceiveActorBeginOverlap` _returnvalue))))
    (else
      (`/Engine/EditorBlueprintResources/StandardMacros.IsValid` (stale `self.ReceiveActorBeginOverlap` _returnvalue_2)
        (:`Is Valid`
          (`Widget.RemoveFromParent` (stale `self.ReceiveActorBeginOverlap` _returnvalue_2)))))))

(fn `Close`
  (`SceneComponent.K2_SetRelativeLocation` (`self.Cube1`) (0.0 0.0 0.0) false false))

(fn `Open`
  (`SceneComponent.K2_SetRelativeLocation` (`self.Cube1`) (`self.OpenPosition`) false false)
  (`GameplayStatics.PlaySoundAtLocation` "/Game/Audio/OpenDoorWithKey.OpenDoorWithKey" (`SceneComponent.K2_GetComponentLocation` (`self.DefaultSceneRoot`)) (struct) 1.0 1.0 0.0 null null null)
  (`PrimitiveComponent.SetMaterial` (`self.Cube1`) 1 "/Game/Materials/M_Laserdoors.M_Laserdoors")
  (`PrimitiveComponent.SetMaterial` (`self.Cube`) 1 "/Game/Materials/M_Laserdoors.M_Laserdoors"))

(fn `UserConstructionScript`)